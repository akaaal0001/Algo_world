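; BP_Stack is a last-in, first-out stack of number blocks, built on an array with add, pop and peek functions.
; AddToStack rejects invalid, zero-numbered or duplicate blocks, while PeekStack reports the top number, using -1 when empty.
; PopFromStack, gated on StackCount, returns the top block to its original transform, re-enables its collision and updates the count.
; Successful adds and pops call CallStackChanged, but only pop updates StackCount here.
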(fn `AddToStack`
  (params (NumberBlock :type "/Game/Big0Arena/Blueprints/BP_NumberBlock Object Reference"))
  (returns (AddedSuccessfully :type Boolean))
  (bind _blockstack (`self.BlockStack`))
  (`/Engine/EditorBlueprintResources/StandardMacros.IsValid` NumberBlock
    (:`Is Valid`
      (if (!= (`/Game/Big0Arena/Blueprints/BP_NumberBlock.BlockNumber` NumberBlock) 0)
        (if (`KismetArrayLibrary.Array_Contains` _blockstack NumberBlock)
          _
          (else
            (`KismetArrayLibrary.Array_Add` _blockstack NumberBlock)
            (`self.StackChanged`)
            (return true)))))
    (:`Is Not Valid`
      _))
  (return false))

(fn `PeekStack`
  (returns (TopNumber :type Integer) (`Top Block` :type "/Game/Big0Arena/Blueprints/BP_NumberBlock Object Reference"))
  (bind _returnvalue (`KismetArrayLibrary.Array_Length` (`self.BlockStack`)))
  (bind _output (`|GetArrayItem` (`self.BlockStack`) (- _returnvalue 1)))
  (bind _blocknumber (`/Game/Big0Arena/Blueprints/BP_NumberBlock.BlockNumber` _output))
  (if (> _returnvalue 0)
    (`/Engine/EditorBlueprintResources/StandardMacros.IsValid` _output
      (:`Is Valid`
        (set `self.TopNumber` _blocknumber)
        (return _blocknumber null)))
    (else
      (bind _output_get (set `self.TopNumber` -1))
      (return _output_get _output))))

(fn `PopFromStack`
  (returns (`Popped Block` :type "/Game/Big0Arena/Blueprints/BP_NumberBlock Object Reference"))
  (bind _blockstack (`self.BlockStack`))
  (bind _returnvalue (`KismetArrayLibrary.Array_LastIndex` _blockstack))
  (bind _output (`|GetArrayItem` _blockstack _returnvalue))
  (if (> (`self.StackCount`) 0)
    (bind _output_get (set `self.ActorToPop` _output))
    (`self.K2_SetActorTransform` _output (`/Game/Big0Arena/Blueprints/BP_NumberBlock.OriginalTransform` _output) false false)
    (`PrimitiveComponent.SetCollisionEnabled` (`/Game/Big0Arena/Blueprints/BP_NumberBlock.BlockMesh` _output) "QueryAndPhysics")
    (`KismetArrayLibrary.Array_Remove` _blockstack _returnvalue)
    (`/Engine/EditorBlueprintResources/StandardMacros.IsValid` _output_get
      (:`Is Valid`
        (bind _output_get_2 (set `self.StackCount` (`KismetArrayLibrary.Array_Length` _blockstack)))
        (`self.StackChanged`)
        (return _output_get)))))

(fn `UserConstructionScript`)