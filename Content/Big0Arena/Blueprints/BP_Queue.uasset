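; BP_Queue is an actor Blueprint that implements a queue of number blocks for Big0Arena.
; Enqueue appends a block to the BlockQueue array and increments QueueCount; Dequeue removes index 0 and decrements it when the count is above zero.
; Dequeue reads index 0 after the removal, so it returns the new front rather than the removed block.
; The event graph and construction script are empty.
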(fn `Dequeue`
  (returns (NumberBlock :type "/Game/Big0Arena/Blueprints/BP_NumberBlock Object Reference"))
  (bind _queuecount (`self.QueueCount`))
  (bind _blockqueue (`self.BlockQueue`))
  (if (> _queuecount 0)
    (`KismetArrayLibrary.Array_Remove` _blockqueue)
    (set `self.QueueCount` (- _queuecount 1))
    (return (`|GetArrayItem` _blockqueue))))

(fn `Enqueue`
  (params (NumberBlock :type "/Game/Big0Arena/Blueprints/BP_NumberBlock Object Reference"))
  (`KismetArrayLibrary.Array_Add` (`self.BlockQueue`) NumberBlock)
  (set `self.QueueCount` (+ (`self.QueueCount`) 1))
  (return))

(fn `UserConstructionScript`)