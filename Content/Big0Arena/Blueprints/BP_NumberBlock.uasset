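; BP_NumberBlock is a block actor that shows a random two-digit number and can be moved onto a stack.
; BeginPlay picks the number and writes it to the block's text, and SetHighlighted toggles custom depth rendering on the mesh.
; MoveToStack saves the original transform, registers the block with StackReference, then places it above the StackSlot at a height scaled by the stack count.
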(event `Set Highlighted`
  (params (Highlighted :type Boolean))
  (`PrimitiveComponent.SetRenderCustomDepth` (`self.BlockMesh`) Highlighted))

(event `self.ReceiveBeginPlay`
  (set `self.BlockNumber` (`KismetMathLibrary.RandomIntegerInRange` 10 99))
  (`TextRenderComponent.K2_SetText` (`self.NumberText`) (`KismetTextLibrary.Conv_IntToText` (`self.BlockNumber`))))

(fn `MoveToStack`
  (bind _stackreference (`self.StackReference`))
  (set `self.OriginalTransform` (`self.GetTransform`))
  (`/Game/Big0Arena/Blueprints/BP_Stack.AddToStack` (`self.StackReference`) self)
  (`self.K2_SetActorLocation` (`KismetMathLibrary.MakeVector` (.x (`SceneComponent.K2_GetComponentLocation` (`/Game/Big0Arena/Blueprints/BP_Stack.StackSlot` _stackreference))) (.y (`SceneComponent.K2_GetComponentLocation` (`/Game/Big0Arena/Blueprints/BP_Stack.StackSlot` _stackreference))) (+ (.z (`SceneComponent.K2_GetComponentLocation` (`/Game/Big0Arena/Blueprints/BP_Stack.StackSlot` _stackreference))) (* (`/Game/Big0Arena/Blueprints/BP_Stack.StackCount` _stackreference) 85)))))

(fn `UserConstructionScript`)